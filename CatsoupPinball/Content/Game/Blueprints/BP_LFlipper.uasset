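; BP_LFlipper is a left flipper actor that swings between a rest angle and a flip angle on press and release events.
; The press and release events set a Flip flag, which Tick uses to run a clamped timer up or down, rising 1.5 times faster than it falls.
; Tick turns that timer into an alpha and sets the actor's relative rotation by shortest-path lerp, without sweep or teleport.
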(event Custom|FlipReleased
  (Variables|Default|SetFlip false))

(event Custom|FlipPressed
  (Variables|Default|SetFlip true))

(event EventTick
  (params (DeltaSeconds :type Float%20%28single-precision%29))
  (bind _flipduration (Variables|Default|GetFlipDuration))
  (if (Variables|Default|GetFlip)
    (Variables|Default|SetCurrentTime (Math|Float|Clamp(Float) (+ (* DeltaSeconds 1.5) (Variables|Default|GetCurrentTime)) 0.0 _flipduration))
    (else
      (Variables|Default|SetCurrentTime (Math|Float|Clamp(Float) (- (Variables|Default|GetCurrentTime) DeltaSeconds) 0.0 _flipduration))))
  (Transformation|SetActorRelativeRotation (Math|Rotator|Lerp(Rotator) (Variables|Default|GetRestAngle) (Variables|Default|GetFlipAngle) (Math|Float|Clamp(Float) (/ (Variables|Default|GetCurrentTime) (Variables|Default|GetFlipDuration))) true)))

(fn ConstructionScript)