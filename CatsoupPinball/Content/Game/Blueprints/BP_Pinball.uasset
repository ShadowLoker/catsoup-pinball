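; BP_Pinball is the pinball actor and drives its FMOD rolling and impact audio.
; Each Tick feeds the ball's velocity magnitude into both a global Speed parameter and the Rolling sound's Speed parameter, restarting that sound whenever it stops.
; Ball hits play a collision event attached to the FMODAudio component, gated by minimum impulse, speed along the hit normal and a cooldown to filter out weak or repeated contacts.
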(event OnComponentHit(Ball)
  (params (HitComponent :type Primitive%20Component%20Object%20Reference) (OtherActor :type Actor%20Object%20Reference) (OtherComp :type Primitive%20Component%20Object%20Reference) (NormalImpulse :type Vector :default "0, 0, 0") (Hit :type Hit%20Result%20Structure%20%28by%20ref%29))
  ;[0.15 0.15 0.15 0.5] Audio On Impact
  ;;[0.15 0.15 0.15 0.5] Check Impulse
  (if (> (Math|Vector|VectorLength NormalImpulse) (Variables|Default|GetMinImpulse))
    ;;[0.15 0.15 0.15 0.5] Check Normal Speed
    (if (> (Math|Float|Absolute(Float) (Math|Vector|DotProduct (Transformation|GetVelocity) (.normal Hit))) (Variables|Default|GetMinNormalSpeed))
      ;;[0.15 0.15 0.15 0.5] Wait For Cooldown
      (if (> (- (Utilities|Time|GetGameTimeinSeconds) (Variables|Default|GetLastImpact)) (Variables|Default|GetCooldown))
        ;;[0.15 0.15 0.15 0.5] Update Last Impact AND Play Audio
        (Variables|Default|SetLastImpact (Utilities|Time|GetGameTimeinSeconds))
        (Class|FMODBlueprintStatics|PlayEventAttached "/Game/FMOD/Events/VFX/Ball/BallCollision.BallCollision" (Variables|Default|GetFMODAudio) "None" "0, 0, 0" "KeepRelativeOffset")))))

(event EventBeginPlay)

(event Collision|EventActorBeginOverlap
  (params (OtherActor :type Actor%20Object%20Reference)))

(event EventTick
  (params (DeltaSeconds :type Float%20%28single-precision%29))
  (bind _returnvalue (Transformation|GetVelocity))
  (bind _rolling (Variables|Default|GetRolling))
  (bind _returnvalue_2 (Math|Vector|VectorLength _returnvalue))
  (Class|FMODBlueprintStatics|SetGlobalParameterbyName "Speed" _returnvalue_2)
  (Class|FMODAudioComponent|SetParameter _rolling "Speed" _returnvalue_2)
  (bind _returnvalue_3 (Class|FMODAudioComponent|IsPlaying _rolling))
  (if (not _returnvalue_3)
    (Class|FMODAudioComponent|Play _rolling)))

(fn ConstructionScript)