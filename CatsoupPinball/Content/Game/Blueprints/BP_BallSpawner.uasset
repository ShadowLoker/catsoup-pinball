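; BP_BallSpawner is a pinball actor that spawns the ball and handles drains.
; It spawns a BP_Pinball at its own transform on BeginPlay.
; When a ball overlaps the BallDestroyer component, it destroys that ball and spawns a replacement.
; It then appends the current score to GM_Pinball's ScoreHistory and resets the points through the game mode.
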(event OnComponentBeginOverlap(BallDestroyer)
  (params (OverlappedComponent :type Primitive%20Component%20Object%20Reference) (OtherActor :type Actor%20Object%20Reference) (OtherComp :type Primitive%20Component%20Object%20Reference) (OtherBodyIndex :type Integer) (bFromSweep :type Boolean) (SweepResult :type Hit%20Result%20Structure%20%28by%20ref%29))
  (bind _asbp_pinball (Utilities|Casting|CastToBP_Pinball OtherActor))
  (Actor|DestroyActor _asbp_pinball)
  (CallFunction|SpawnBall)
  (bind _asgm_pinball (Utilities|Casting|CastToGM_Pinball (Game|GetGameMode)))
  (Utilities|Array|Add (Variables|/Game/Game/System/GM_Pinball.GM_Pinball_C|GetScoreHistory _asgm_pinball) (Variables|/Game/Game/System/GM_Pinball.GM_Pinball_C|GetScore _asgm_pinball))
  (Default|ResetPoints _asgm_pinball))

(event Custom|SpawnBall
  (Game|SpawnActorfromClass "/Game/Game/Blueprints/BP_Pinball.BP_Pinball_C" (Transformation|GetActorTransform) "Undefined" "MultiplyWithRoot" 0 0))

(event EventBeginPlay
  (CallFunction|SpawnBall))

(fn ConstructionScript)