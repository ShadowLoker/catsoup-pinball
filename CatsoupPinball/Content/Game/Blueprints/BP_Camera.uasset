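; BP_Camera is the pinball table camera, which also serves as the player's input handler.
; On BeginPlay it becomes player 0's view target and enables input on itself.
; Enhanced Input actions for the left and right buttons press and release the referenced flippers, and the launcher action charges and releases the plunger.
; Canceled and Completed share the same release path.
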(event Input|EnhancedActionEvents|EnhancedInputActionIA_LeftButton
  (params (ActionValue :type Boolean) (ElapsedSeconds :type Float%20%28double-precision%29) (TriggeredSeconds :type Float%20%28double-precision%29) (InputAction :type Input%20Action%20Object%20Reference :default "/Game/Game/System/Inputs/IA_LeftButton.IA_LeftButton"))
  (bind _leftflippers (Variables|Default|GetLeftFlippers))
  (:Started
    (Default|FlipPressed _leftflippers))
  (:Canceled
    (Default|FlipReleased _leftflippers :!label _label))
  (:Completed
    (goto _label)))

(event Input|EnhancedActionEvents|EnhancedInputActionIA_RightButton
  (params (ActionValue :type Boolean) (ElapsedSeconds :type Float%20%28double-precision%29) (TriggeredSeconds :type Float%20%28double-precision%29) (InputAction :type Input%20Action%20Object%20Reference :default "/Game/Game/System/Inputs/IA_RightButton.IA_RightButton"))
  (bind _rightflippers (Variables|Default|GetRightFlippers))
  (:Started
    (Default|FlipPressed _rightflippers))
  (:Canceled
    (Default|FlipReleased _rightflippers :!label _label))
  (:Completed
    (goto _label)))

(event Input|EnhancedActionEvents|EnhancedInputActionIA_Launcher
  (params (ActionValue :type Boolean) (ElapsedSeconds :type Float%20%28double-precision%29) (TriggeredSeconds :type Float%20%28double-precision%29) (InputAction :type Input%20Action%20Object%20Reference :default "/Game/Game/System/Inputs/IA_Launcher.IA_Launcher"))
  (bind _plunger (Variables|Default|GetPlunger))
  (:Started
    (Default|Charge _plunger))
  (:Canceled
    (Default|Release _plunger :!label _label))
  (:Completed
    (goto _label)))

(event EventBeginPlay
  (bind _returnvalue (Game|GetPlayerController 0))
  (Game|Player|SetViewTargetwithBlend _returnvalue self 0.0 "VTBlend_Linear" 0.0 false)
  (Input|EnableInput _returnvalue))

(event Collision|EventActorBeginOverlap
  (params (OtherActor :type Actor%20Object%20Reference)))

(event EventTick
  (params (DeltaSeconds :type Float%20%28single-precision%29)))

(fn ConstructionScript)