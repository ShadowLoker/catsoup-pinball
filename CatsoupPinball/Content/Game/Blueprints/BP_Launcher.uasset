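; BP_Launcher is a pinball launcher actor that fires balls along its arrow's direction.
; An actor overlap starts a two-second delay, then calls the Launch event.
; Launch finds every BP_Pinball overlapping its sphere and applies an impulse to each root primitive component, scaled by LaunchForce along the Arrow's forward vector.
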(event Custom|Launch
  (for _array_element (Collision|GetOverlappingActors (Variables|Default|GetSphere) "/Game/Game/Blueprints/BP_Pinball.BP_Pinball_C" :!class /Script/Engine.PrimitiveComponent)
    (bind _asprimitive_component (Utilities|Casting|CastToPrimitiveComponent (Variables|/Script/Engine.Actor|GetRootComponent _array_element)))
    (Physics|AddImpulse _asprimitive_component (* (Variables|Default|GetLaunchForce) (Math|Vector|GetForwardVector (Variables|Default|GetArrow))) "None" false)))

(event EventBeginPlay)

(event Collision|EventActorBeginOverlap
  (params (OtherActor :type Actor%20Object%20Reference))
  (Utilities|FlowControl|Delay 2.0)
  (CallFunction|Launch))

(event EventTick
  (params (DeltaSeconds :type Float%20%28single-precision%29)))

(fn ConstructionScript)