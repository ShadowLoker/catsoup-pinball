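; BP_ScoreOnHitComponent is an actor component that awards points when a pinball strikes its owning actor.
; On BeginPlay it binds to the owner's OnActorHit event.
; Each hit counts only if the other actor is exactly BP_Pinball and the impulse magnitude exceeds MinImpulse, in which case it adds Points through the GM_Pinball game mode.
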(event Custom|HandleHit
  (params (SelfActor :type Actor%20Object%20Reference) (OtherActor :type Actor%20Object%20Reference) (NormalImpulse :type Vector) (Hit :type Hit%20Result%20Structure%20%28by%20ref%29))
  (if (and (== (Utilities|GetClass OtherActor) "/Game/Game/Blueprints/BP_Pinball.BP_Pinball_C") (> (Math|Vector|VectorLength NormalImpulse) (Variables|Default|GetMinImpulse)))
    (bind _asgm_pinball (Utilities|Casting|CastToGM_Pinball (Game|GetGameMode)))
    (Default|AddPoints _asgm_pinball (Variables|Default|GetPoints))))

(event EventBeginPlay
  (Collision|AssignOnActorHit (Components|GetOwner) (delegate Custom|HandleHit)))

(event EventTick
  (params (DeltaSeconds :type Float%20%28single-precision%29)))