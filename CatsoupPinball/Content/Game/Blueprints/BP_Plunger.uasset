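; BP_Plunger is a plunger actor that pulls its static mesh toward a charge position while charging and returns it on release.
; Charge and Release events toggle a flag that Tick reads to raise or lower a clamped timer, with the return running five times faster.
; Each tick, the timer's fraction of the release time interpolates the mesh's relative location between rest and charge positions, without sweep or teleport.
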(event Custom|Charge
  (Variables|Default|SetCharging true))

(event Custom|Release
  (Variables|Default|SetCharging false))

(event EventBeginPlay)

(event Collision|EventActorBeginOverlap
  (params (OtherActor :type Actor%20Object%20Reference)))

(event EventTick
  (params (DeltaSeconds :type Float%20%28single-precision%29))
  (if (Variables|Default|GetCharging)
    (Variables|Default|SetCurrentTime (Math|Float|Clamp(Float) (+ (Variables|Default|GetCurrentTime) DeltaSeconds) 0.0 (Variables|Default|GetReleaseTime)))
    (else
      (Variables|Default|SetCurrentTime (Math|Float|Clamp(Float) (- (Variables|Default|GetCurrentTime) (* DeltaSeconds 5.0)) 0.0 (Variables|Default|GetReleaseTime)))))
  (Transformation|SetRelativeLocation (Variables|Default|GetStaticMesh) (Math|Vector|Lerp(Vector) (Variables|Default|GetRestPosition) (Variables|Default|GetChargePosition) (/ (Variables|Default|GetCurrentTime) (Variables|Default|GetReleaseTime))) false false))

(fn ConstructionScript)