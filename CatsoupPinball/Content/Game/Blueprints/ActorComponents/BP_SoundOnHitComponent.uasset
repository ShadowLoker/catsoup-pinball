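; BP_SoundOnHitComponent is an actor component that plays an FMOD sound when a pinball hits its owning actor.
; On BeginPlay it binds to the owner's hit event and adds an FMOD audio component set to a configurable event reference.
; On a hit by BP_Pinball, the sound plays only if the impulse magnitude exceeds the MinImpulse threshold read from the GM_Pinball game mode.
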(event Custom|HandleHit
  (params (SelfActor :type Actor%20Object%20Reference) (OtherActor :type Actor%20Object%20Reference) (NormalImpulse :type Vector) (Hit :type Hit%20Result%20Structure%20%28by%20ref%29))
  (if (== "/Game/Game/Blueprints/BP_Pinball.BP_Pinball_C" (Utilities|GetClass OtherActor))
    (bind _asgm_pinball (Utilities|Casting|CastToGM_Pinball (Game|GetGameMode)))
    (if (< (Variables|/Game/Game/System/GM_Pinball.GM_Pinball_C|GetMinImpulse _asgm_pinball) (Math|Vector|VectorLength NormalImpulse))
      (Class|FMODAudioComponent|Play (Variables|Default|GetFMODComp)))))

(event EventBeginPlay
  (bind _returnvalue (Components|GetOwner))
  (Collision|AssignOnActorHit _returnvalue (delegate Custom|HandleHit))
  (bind _returnvalue_2 (Game|AddComponentbyClass _returnvalue "/Script/FMODStudio.FMODAudioComponent" false))
  (bind _output_get (Variables|Default|SetFMODComp _returnvalue_2))
  (Class|FMODAudioComponent|SetEvent _output_get (Variables|Default|GetFMODEventReference)))