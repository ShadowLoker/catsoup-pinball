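; BP_ScoreOnHitComponent is an actor component that awards points when a pinball hits its owning actor.
; On BeginPlay it binds a handler to the owner's OnActorHit event and reacts only to actors whose class is exactly BP_Pinball.
; Hits with an impulse magnitude above GM_Pinball's MinImpulse pass the component's Points to the game mode's RegisterScoreHit.
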(event Custom|HandleHit
  (params (SelfActor :type Actor%20Object%20Reference) (OtherActor :type Actor%20Object%20Reference) (NormalImpulse :type Vector) (Hit :type Hit%20Result%20Structure%20%28by%20ref%29))
  (if (== "/Game/Game/Blueprints/BP_Pinball.BP_Pinball_C" (Utilities|GetClass OtherActor))
    (bind _asgm_pinball (Utilities|Casting|CastToGM_Pinball (Game|GetGameMode)))
    (if (< (Variables|/Game/Game/System/GM_Pinball.GM_Pinball_C|GetMinImpulse _asgm_pinball) (Math|Vector|VectorLength NormalImpulse))
      (Default|RegisterScoreHit _asgm_pinball (Variables|Default|GetPoints)))))

(event EventBeginPlay
  (Collision|AssignOnActorHit (Components|GetOwner) (delegate Custom|HandleHit)))

(event EventTick
  (params (DeltaSeconds :type Float%20%28single-precision%29)))