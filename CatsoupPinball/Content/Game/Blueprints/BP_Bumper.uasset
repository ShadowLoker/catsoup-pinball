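; BP_Bumper is a pinball bumper that kicks the ball away when its capsule is hit.
; On hit it applies a velocity-change impulse to the BP_Pinball ball along the normalized hit normal, scaled by Force.
; A timeline also rescales the bumper's X and Y as a pop animation for any hit, while the sound event is an empty stub.
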(event OnComponentHit(Capsule)
  (params (HitComponent :type Primitive%20Component%20Object%20Reference) (OtherActor :type Actor%20Object%20Reference) (OtherComp :type Primitive%20Component%20Object%20Reference) (NormalImpulse :type Vector :default "0, 0, 0") (Hit :type Hit%20Result%20Structure%20%28by%20ref%29))
  (CallFunction|HitImpulse OtherActor NormalImpulse)
  (CallFunction|HitSound)
  (CallFunction|HitAnim))

(event Custom|HitAnim
  (bind _size (Timeline|Animation PlayFromStart)
    (:Update
      (Transformation|SetRelativeScale3D (Variables|Default|GetBumper) (Math|Vector|MakeVector _size _size 0.3)))))

(event Custom|HitSound)

(event Custom|HitImpulse
  (params (Other%20Actor :type Object%20Object%20Reference) (Normal%20Impulse :type Vector))
  (bind _asbp_pinball (Utilities|Casting|CastToBP_Pinball Other%20Actor))
  (Physics|AddImpulse (Variables|/Game/Game/Blueprints/BP_Pinball.BP_Pinball_C|GetBall _asbp_pinball) (* (Math|Vector|Normalize Normal%20Impulse) (Variables|Default|GetForce)) "None" true))

(fn ConstructionScript)