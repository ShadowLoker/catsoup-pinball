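; Pinball game mode that tracks score, session high score and a decaying combo multiplier, plays music, and quits on Enter or Escape.
; Each registered score raises the combo, adds multiplied points and restarts a looping timer that drains the meter, dropping one combo step per empty window.
; Resetting points records the high score and clears score and combo.
; Changes broadcast through dispatchers, and scoring feeds the multiplier to a global FMOD audio parameter.
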(event Custom|RegisterScore
  (params (BasePoints :type Integer))
  (Math|Integer|IncrementInt (Variables|Default|GetComboCount)
    (:%20%20
      (CallFunction|IncreaseScore (* (Utilities|ComboMultiplier) BasePoints))
      (CallFunction|ResetComboMeter)
      (Default|CallOnComboChanged (Utilities|ComboMultiplier) (Utilities|ComboMeterPercentage))
      (Utilities|Time|ClearandInvalidateTimerbyHandle (Variables|Default|GetComboTickHandle))
      (bind _returnvalue (Utilities|Time|SetTimerbyEvent (delegate Custom|ComboDecayTick) (Variables|Default|GetComboTickInterval) true))
      (Variables|Default|SetComboTickHandle _returnvalue))))

(event Custom|ComboDecayTick
  (if (<= (Variables|Default|GetComboCount) 0)
    (Variables|Default|SetComboCount 0)
    (Utilities|Time|ClearandInvalidateTimerbyHandle (Variables|Default|GetComboTickHandle))
    (else
      (bind _output_get (Variables|Default|SetComboMeter (- (Variables|Default|GetComboMeter) (Variables|Default|GetComboTickInterval))))
      (if (<= _output_get 0.0)
        (bind _returnvalue (CallFunction|DecreaseComboCount))
        (if (> _returnvalue 0)
          (CallFunction|ResetComboMeter)
          (else
            (Variables|Default|SetComboMeter 0.0)
            (Utilities|Time|ClearandInvalidateTimerbyHandle (Variables|Default|GetComboTickHandle))))
        (Default|CallOnComboChanged (Utilities|ComboMultiplier) (Utilities|ComboMeterPercentage))
        (else
          (Default|CallOnComboChanged (Utilities|ComboMultiplier) (Utilities|ComboMeterPercentage)))))))

(event Custom|ResetPoints
  (CallFunction|RegisterHighScore)
  (CallFunction|ResetScore)
  (CallFunction|ResetCombo))

(event EventBeginPlay
  (Class|FMODBlueprintStatics|PlayEvent2D "/Game/FMOD/Events/Music.Music"))

(event EventTick
  (params (DeltaSeconds :type Float%20%28single-precision%29)))

(event Input|KeyboardEvents|Escape
  (params (Key :type Key%20Structure :default "None"))
  (:Pressed
    (Game|QuitGame 0 "Quit" false)))

(event Input|KeyboardEvents|Enter
  (params (Key :type Key%20Structure :default "None"))
  (:Pressed
    (Game|QuitGame 0 "Quit" false)))

(fn ConstructionScript)

(fn DecreaseComboCount
  (bind _output_get (Variables|Default|SetComboCount (Math|Integer|Clamp(Integer) (- (Variables|Default|GetComboCount) 1) 0 (- (Utilities|Array|Length (Variables|Default|GetMultipliers)) 1))))
  (return _output_get))

(fn ResetCombo
  (Utilities|Time|ClearandInvalidateTimerbyHandle (Variables|Default|GetComboTickHandle))
  (Variables|Default|SetComboMeter 0.0)
  (bind _output_get (Variables|Default|SetComboCount 0))
  (Default|CallOnComboChanged _output_get (Utilities|ComboMeterPercentage)))

(fn RegisterHighScore
  (if (< (Variables|Default|GetHighscore) (Variables|Default|GetScore))
    (bind _output_get (Variables|Default|SetHighscore (Variables|Default|GetScore)))
    (Default|CallOnHighscoreChanged _output_get)))

(fn ResetScore
  (bind _output_get (Variables|Default|SetScore 0))
  (Default|CallOnScoreChanged _output_get))

(fn IncreaseScore
  (params (A :type Integer))
  (bind _output_get (Variables|Default|SetScore (+ A (Variables|Default|GetScore))))
  (Default|CallOnScoreChanged _output_get)
  (Class|FMODBlueprintStatics|SetGlobalParameterbyName "Multiplier" (Math|Conversions|ToFloat(Integer) (Utilities|ComboMultiplier)))
  (Class|FMODBlueprintStatics|PlayEvent2D "/Game/FMOD/Events/VFX/Bonus/Multiplier.Multiplier"))

(fn ResetComboMeter
  (Variables|Default|SetComboMeter (Variables|Default|GetComboWindow)))